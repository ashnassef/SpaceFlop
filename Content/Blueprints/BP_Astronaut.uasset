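; Physics-simulated astronaut that randomly takes a male or female mesh and physics asset, with collision-driven impact and sliding audio.
; The random pick runs in the construction script and again at BeginPlay.
; The first mesh hit lazily spawns and attaches three audio actors: impact, slide one-shots and looping slide.
; Each hit feeds them impulse, hit data, cached tick delta time and velocity values calculated by the impact actor.
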(event `self.SkeletalMesh.OnComponentHit`
  (params (HitComponent :type "PrimitiveComponent Object Reference") (OtherActor :type "Actor Object Reference") (OtherComp :type "PrimitiveComponent Object Reference") (NormalImpulse :type "Vector Structure") (Hit :type "HitResult Structure (by ref)"))
  ;[1 1 1] Impact sounds
  (set `self.normalImpulse` NormalImpulse)
  (set `self.hitResult` Hit)
  (if (`self.spawnedCollider`)
    (`/UnrealAudioKit/AudioActor/BP_AA_Collision.calculateVelocityValues` (`self.collisionSound`) (`self.normalImpulse`) (`self.hitResult`) (`self.SkeletalMesh`))
    (set `self.audioVelocityVals` (`/UnrealAudioKit/AudioActor/BP_AA_Collision.velocityValues` (`self.collisionSound`)))
    (`/UnrealAudioKit/AudioActor/BP_AA_Collision.setCollisionValues` (`self.collisionSound`) (`self.normalImpulse`) (`self.hitResult`) null (`self.SkeletalMesh`) (`self.deltaTime`) (`self.audioVelocityVals`))
    (else
      (bind _returnvalue (`|SpawnActorFromClass` "/UnrealAudioKit/AudioActor/BP_AA_Collision.BP_AA_Collision_C" (`SceneComponent.K2_GetComponentToWorld` (`self.SkeletalMesh`)) "AlwaysSpawn" "OverrideRootScale" self null))
      (`/UnrealAudioKit/AudioActor/BP_AA_Collision.calculateVelocityValues` _returnvalue (`self.normalImpulse`) (`self.hitResult`) (`self.SkeletalMesh`))
      (set `self.collisionSound` _returnvalue)
      (set `self.audioVelocityVals` (`/UnrealAudioKit/AudioActor/BP_AA_Collision.velocityValues` _returnvalue))
      (`AudioComponent.SetSound` (`/UnrealAudioKit/AudioActor/BP_AudioActor.AudioComponent` _returnvalue) "/Game/Audio/Cues/Cue_Impact.Cue_Impact")
      (`self.K2_AttachToComponent` _returnvalue (`self.SkeletalMesh`) "None" "KeepRelative" "KeepRelative" "KeepRelative" true)
      (`self.K2_AttachToComponent` (`self.collisionSound`) (`self.SkeletalMesh`) "None" "KeepRelative" "KeepRelative" "KeepRelative" true)
      (`/UnrealAudioKit/AudioActor/BP_AA_Collision.setCollisionValues` _returnvalue (`self.normalImpulse`) (`self.hitResult`) null (`self.SkeletalMesh`) (`self.deltaTime`) (`self.audioVelocityVals`))
      (set `self.spawnedCollider` true)))
  ;[1 1 1] Sliding one shot sounds
  (if (`self.spawnedSlider`)
    (`/UnrealAudioKit/AudioActor/BP_AA_Slide.setCollisionValues` (`self.slideSound`) (`self.normalImpulse`) (`self.hitResult`) null (`self.SkeletalMesh`) (`self.deltaTime`) (`self.audioVelocityVals`))
    (else
      (bind _returnvalue_2 (`|SpawnActorFromClass` "/UnrealAudioKit/AudioActor/BP_AA_Slide.BP_AA_Slide_C" (`SceneComponent.K2_GetComponentToWorld` (`self.SkeletalMesh`)) "AlwaysSpawn" "OverrideRootScale" self null))
      (`AudioComponent.SetSound` (`/UnrealAudioKit/AudioActor/BP_AudioActor.AudioComponent` _returnvalue_2) "/Game/Audio/Cues/Cue_SlideOneShots.Cue_SlideOneShots")
      (bind _output_get (set `self.slideSound` _returnvalue_2))
      (`self.K2_AttachToComponent` _output_get (`self.SkeletalMesh`) "None" "KeepRelative" "KeepRelative" "KeepRelative" true)
      (`self.K2_AttachToComponent` (`self.slideSound`) (`self.SkeletalMesh`) "None" "KeepRelative" "KeepRelative" "KeepRelative" true)
      (`/UnrealAudioKit/AudioActor/BP_AA_Slide.setCollisionValues` _returnvalue_2 (`self.normalImpulse`) (`self.hitResult`) null (`self.SkeletalMesh`) (`self.deltaTime`) (`self.audioVelocityVals`))
      (set `self.spawnedSlider` true)))
  ;[1 1 1] Looping slide sound
  (if (`self.spawnedSliderPad`)
    (`/UnrealAudioKit/AudioActor/BP_AA_Slide.setCollisionValues` (`self.slideLoopSound`) (`self.normalImpulse`) (`self.hitResult`) null (`self.SkeletalMesh`) (`self.deltaTime`) (`self.audioVelocityVals`))
    (else
      (bind _returnvalue_3 (`|SpawnActorFromClass` "/UnrealAudioKit/AudioActor/BP_AA_Slide.BP_AA_Slide_C" (`SceneComponent.K2_GetComponentToWorld` (`self.SkeletalMesh`)) "AlwaysSpawn" "OverrideRootScale" self null))
      (`AudioComponent.SetSound` (`/UnrealAudioKit/AudioActor/BP_AudioActor.AudioComponent` _returnvalue_3) "/Game/Audio/Cues/Cue_Slide.Cue_Slide")
      (bind _output_get_2 (set `self.slideLoopSound` _returnvalue_3))
      (set `/UnrealAudioKit/AudioActor/BP_AA_Slide.loopingSound` true _returnvalue_3)
      (`self.K2_AttachToComponent` _output_get_2 (`self.SkeletalMesh`) "None" "KeepRelative" "KeepRelative" "KeepRelative" true)
      (`self.K2_AttachToComponent` (`self.slideLoopSound`) (`self.SkeletalMesh`) "None" "KeepRelative" "KeepRelative" "KeepRelative" true)
      (`/UnrealAudioKit/AudioActor/BP_AA_Slide.setCollisionValues` _returnvalue_3 (`self.normalImpulse`) (`self.hitResult`) null (`self.SkeletalMesh`) (`self.deltaTime`) (`self.audioVelocityVals`))
      (set `self.spawnedSliderPad` true))))

(event `self.ReceiveBeginPlay`
  (if (`KismetMathLibrary.RandomBool`)
    (`SkinnedMeshComponent.SetSkinnedAssetAndUpdate` (`self.SkeletalMesh`) "/Game/Assets/Meshes/SkeletalMesh_AstronautFemale.SkeletalMesh_AstronautFemale" true)
    (`SkinnedMeshComponent.SetPhysicsAsset` (`self.SkeletalMesh`) "/Game/Assets/Meshes/PhysicsAsset_AstronautFemale.PhysicsAsset_AstronautFemale" true)
    (else
      (`SkinnedMeshComponent.SetSkinnedAssetAndUpdate` (`self.SkeletalMesh`) "/Game/Assets/Meshes/SkeletalMesh_AstronautMale.SkeletalMesh_AstronautMale" true)
      (`SkinnedMeshComponent.SetPhysicsAsset` (`self.SkeletalMesh`) "/Game/Assets/Meshes/PhysicsAsset_AstronautMale.PhysicsAsset_AstronautMale" true)))
  (`PrimitiveComponent.SetSimulatePhysics` (`self.SkeletalMesh`) true))

(event `self.ReceiveTick`
  (params (DeltaSeconds :type "Float (single-precision)"))
  (set `self.deltaTime` DeltaSeconds))

(fn `UserConstructionScript`
  (if (`KismetMathLibrary.RandomBool`)
    (`SkinnedMeshComponent.SetSkinnedAssetAndUpdate` (`self.SkeletalMesh`) "/Game/Assets/Meshes/SkeletalMesh_AstronautFemale.SkeletalMesh_AstronautFemale" true)
    (`SkinnedMeshComponent.SetPhysicsAsset` (`self.SkeletalMesh`) "/Game/Assets/Meshes/PhysicsAsset_AstronautFemale.PhysicsAsset_AstronautFemale" true)
    (else
      (`SkinnedMeshComponent.SetSkinnedAssetAndUpdate` (`self.SkeletalMesh`) "/Game/Assets/Meshes/SkeletalMesh_AstronautMale.SkeletalMesh_AstronautMale" true)
      (`SkinnedMeshComponent.SetPhysicsAsset` (`self.SkeletalMesh`) "/Game/Assets/Meshes/PhysicsAsset_AstronautMale.PhysicsAsset_AstronautMale" true)))
  (`PrimitiveComponent.SetSimulatePhysics` (`self.SkeletalMesh`) true))